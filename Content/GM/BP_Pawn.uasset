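; BP_Pawn is a player pawn that handles start and restart input and plays crash feedback.
; The construction script assigns its camera, spring arm, box and static mesh components to pawn variables.
; Enhanced Input actions call LocalStart, defined outside these graphs, or restart the level through a console command.
; A static mesh overlap with a TriggerVolume plays a 2D Crash sound.
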(event OnComponentBeginOverlap(StaticMesh)
  (params (OverlappedComponent :type Primitive%20Component%20Object%20Reference) (OtherActor :type Actor%20Object%20Reference) (OtherComp :type Primitive%20Component%20Object%20Reference) (OtherBodyIndex :type Integer) (bFromSweep :type Boolean) (SweepResult :type Hit%20Result%20Structure%20%28by%20ref%29))
  (Utilities|Casting|CastToTriggerVolume OtherActor)
  (Audio|PlaySound2D "/Game/Sound/crash.crash" 1.0 1.0 0.0 0 0))

(event Input|EnhancedActionEvents|EnhancedInputActionIA_Start
  (params (ActionValue :type Boolean) (ElapsedSeconds :type Float%20%28double-precision%29) (TriggeredSeconds :type Float%20%28double-precision%29) (InputAction :type Input%20Action%20Object%20Reference :default "/Game/GM/IA_Start.IA_Start"))
  (:Started
    (Class|VDPawn|LocalStart)))

(event Input|EnhancedActionEvents|EnhancedInputActionIA_Return
  (params (ActionValue :type Boolean) (ElapsedSeconds :type Float%20%28double-precision%29) (TriggeredSeconds :type Float%20%28double-precision%29) (InputAction :type Input%20Action%20Object%20Reference :default "/Game/GM/IA_Return.IA_Return"))
  (:Started
    (Development|ExecuteConsoleCommand "RestartLevel" (Game|GetPlayerController 0))))

(event EventBeginPlay)

(event Collision|EventActorBeginOverlap
  (params (OtherActor :type Actor%20Object%20Reference)))

(event EventTick
  (params (DeltaSeconds :type Float%20%28single-precision%29)))

(fn ConstructionScript
  (Variables|Default|SetCamera (Variables|Default|GetBPCamera))
  (Variables|Default|SetMySpringArm (Variables|Default|GetSpringArm))
  (Variables|Default|SetMyBox (Variables|Collision|GetBox))
  (Variables|Default|SetMyMesh (Variables|Default|GetStaticMesh)))